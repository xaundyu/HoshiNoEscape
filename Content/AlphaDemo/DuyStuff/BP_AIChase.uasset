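; BP_AIChase is an enemy pawn that chases the HorrorEngineCharacter player and captures them on contact.
; Pawn sensing triggers AI MoveTo toward the player and keeps a SeePlayer flag true until sightings lapse briefly.
; A capsule hit disables player movement and fires a one-time jumpscare sound and widget, then after a delay pauses the game with a CApted screen.
; A loading-screen level-open chain is left unconnected.
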(event `self.PawnSensing.OnSeePawn`
  (params (Pawn :type "Pawn Object Reference"))
  (bind _ashorror_engine_character (cast `/Game/HorrorEngine/Blueprints/Core/HorrorEngineCharacter` Pawn))
  (`|ExecutionSequence`
    (:`then_0`
      (set `self.SeePlayer?` true)
      (`|AIMoveTo` self (0.0 0.0 0.0) _ashorror_engine_character))
    (:`then_1`
      (`KismetSystemLibrary.RetriggerableDelay` 0.5)
      (set `self.SeePlayer?` false))))

(event `self.CapsuleComponent.OnComponentHit`
  (params (HitComponent :type "PrimitiveComponent Object Reference") (OtherActor :type "Actor Object Reference") (OtherComp :type "PrimitiveComponent Object Reference") (NormalImpulse :type "Vector Structure") (Hit :type "HitResult Structure (by ref)"))
  (bind _ashorror_engine_character (cast `/Game/HorrorEngine/Blueprints/Core/HorrorEngineCharacter` OtherActor))
  (`CharacterMovementComponent.DisableMovement` (`Character.CharacterMovement` _ashorror_engine_character))
  (`/Engine/EditorBlueprintResources/StandardMacros.DoOnce` false
    (:`Completed`
      (`GameplayStatics.PlaySound2D` "/Game/AlphaDemo/DuyStuff/jumpscare_but_not_very_loud.jumpscare_but_not_very_loud" 1.0 1.0 0.0 null null)
      (bind _returnvalue (`|CreateWidget` "/Game/AlphaDemo/DuyStuff/JumpScare.JumpScare_C"))
      (`UserWidget.AddToViewport` _returnvalue 0)
      (`KismetSystemLibrary.Delay` 7.0)
      (`GameplayStatics.SetGamePaused` true)
      (bind _returnvalue_2 (`|CreateWidget` "/Game/AlphaDemo/DuyStuff/CApted.CApted_C"))
      (`UserWidget.AddToViewport` _returnvalue_2 0)
      (`GameplayStatics.SetGamePaused` true))))

(fn `UserConstructionScript`)